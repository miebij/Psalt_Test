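; BP_Fireball_loop_03 is a one-shot fireball explosion effect triggered by the first overlap on its Box component.
; It spawns the PS_fireball_03 emitter at its own transform, then enables physics on the geometry collection actors in NewVar and launches them upward with an impulse.
; A timeline animates the point light's intensity, and the construction script sets that light's color from PColor.
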(event OnComponentBeginOverlap(Box)
  (params (OverlappedComponent :type Primitive%20Component%20Object%20Reference) (OtherActor :type Actor%20Object%20Reference) (OtherComp :type Primitive%20Component%20Object%20Reference) (OtherBodyIndex :type Integer) (bFromSweep :type Boolean) (SweepResult :type Hit%20Result%20Structure%20%28by%20ref%29))
  (bind _returnvalue (Transformation|GetActorTransform))
  (if (not (Variables|Default|GetDone))
    (Variables|Default|SetDone true)
    (Utilities|FlowControl|Sequence
      (:then_0
        (Effects|SpawnEmitteratLocation "/Game/Fire_Explosion_FX/ParticleSystems/PS_fireball_03.PS_fireball_03" (.location _returnvalue) (.rotation _returnvalue) (.scale _returnvalue))
        (for _array_element (Variables|Default|GetNewVar)
          (Physics|SetSimulatePhysics (Variables|/Script/GeometryCollectionEngine.GeometryCollectionActor|GetGeometryCollectionComponent _array_element) true)
          (Physics|AddImpulse (Variables|/Script/GeometryCollectionEngine.GeometryCollectionActor|GetGeometryCollectionComponent _array_element) "0.000000,0.000000,500000.000000" "None" false)))
      (:then_1
        (bind _intensity (Timeline|Timeline_1 PlayFromStart)
          (:Update
            (Rendering|Components|Light|SetIntensity (Variables|Default|GetPointLight) _intensity)))))))

(event EventBeginPlay)

(fn ConstructionScript
  (Rendering|Components|Light|SetLightColor (Variables|Default|GetPointLight) (Variables|Default|GetPColor) true))