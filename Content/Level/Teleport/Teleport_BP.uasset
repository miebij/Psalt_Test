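; Teleport_BP is a level-placed teleport actor that numbers itself, with no teleport logic of its own.
; Its construction script takes the number after the Blueprint's name in the instance's display name, treats values below 2 as 1, then subtracts one.
; The resulting zero-based index replaces the actor's Tags and is shown on its TextRender, so identity depends on instance naming.
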(event EventBeginPlay)

(event Collision|EventActorBeginOverlap
  (params (OtherActor :type Actor%20Object%20Reference)))

(event EventTick
  (params (DeltaSeconds :type Float%20%28single-precision%29)))

(fn ConstructionScript
  (bind _returnvalue (Utilities|GetDisplayName "Teleport_BP"))
  (bind _self self)
  (bind _returnvalue_2 (Utilities|GetDisplayName _self))
  (bind _rights (Utilities|String|Split _returnvalue_2 _returnvalue))
  (bind _returnvalue_3 (Math|Conversions|ToInteger(Byte) _rights))
  (bind _returnvalue_4 (< _returnvalue_3 2))
  (bind _returnvalue_5 (Utilities|String|SelectString "1" _rights _returnvalue_4))
  (bind _returnvalue_6 (Math|Conversions|ToInteger(Byte) _returnvalue_5))
  (bind _returnvalue_7 (- _returnvalue_6 1))
  (bind _returnvalue_8 (Utilities|String|ToString(Integer) _returnvalue_7))
  (Variables|Default|SetTags self (Utilities|Array|MakeArray (Utilities|String|StringToName _returnvalue_8)))
  (Rendering|Components|TextRender|SetText (Variables|Default|GetTextRender) (Utilities|Text|ToText(String) _returnvalue_8)))