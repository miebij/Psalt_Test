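; Blueprint interface for the rope climbing system, declaring the messages that pass rope climbing state between its participants.
; Most functions push data such as grab, swing, jump, climb, rope switching, wall bracing, movement and physics states.
; Hand and foot IK values and per-hand anim notify calls support animation.
; Functions with return values cover swing inputs, overlay state, grab disabling, external start or finish, and rope collection by location and radius.
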(fn EnableRopeClimbing
  (params (Enable_Swinging :type Boolean) (BlendIn :type Float%20%28single-precision%29) (BlendOut :type Float%20%28single-precision%29)))

(fn RopeClimbingStates
  (params (Rope_Detected :type Boolean) (Grab_Rope :type Boolean) (On_Rope :type Boolean)))

(fn RopeClimbUp/Down
  (params (Swinging_Climb_Up :type Boolean) (Swinging_Climb_Down :type Boolean)))

(fn RotationAroundRope
  (params (Rotating_Around_Rope :type Boolean) (RotationDirection :type Float%20%28single-precision%29)))

(fn SwingJump
  (params (Swing_Jump :type Boolean) (JumpZAxis :type Float%20%28single-precision%29) (JumpAngle :type Float%20%28single-precision%29) (OrientToJumpDirection :type Boolean)))

(fn WallBracedState
  (params (Wall_Braced :type Boolean)))

(fn ClimbtoRope
  (params (Rope_Switchig :type Boolean) (MovementAngle :type Float%20%28single-precision%29) (MovementDistance :type Float%20%28single-precision%29)))

(fn RopeExternal
  (params (RopeExternalIn :type Boolean) (RopeExternalOut :type Boolean) (AngleExt :type Float%20%28single-precision%29) (SideExt :type Float%20%28single-precision%29) (DistanceExt :type Float%20%28single-precision%29)))

(fn HandIK
  (params (Hand_IK_R :type Vector) (Hand_IK_L :type Vector)))

(fn HandMovementIK
  (params (Hand_Movement_IK_R :type Vector) (Hand_Movement_IK_L :type Vector)))

(fn LegIK
  (params (Foot_IK_Right :type Vector) (Foot_IK_Left :type Vector)))

(fn NewHandIK
  (params (NewRightHand :type Vector) (NewLeftHand :type Vector)))

(fn AnimNotifyHandR)

(fn AnimNotifyHandL)

(fn SwingingDirection
  (params (Swing_Forward :type Float%20%28single-precision%29) (Swing_Right :type Float%20%28single-precision%29)))

(fn GrabRopeParams
  (params (Time :type Float%20%28single-precision%29) (Angle :type Float%20%28single-precision%29)))

(fn MovementAlpha
  (params (MovementAlpha :type Float%20%28single-precision%29)))

(fn SwingingVelocity
  (params (Perpendicular_Velocity :type Float%20%28single-precision%29)))

(fn WallDistance
  (params (Wall_Distance :type Float%20%28single-precision%29)))

(fn RopeClimbUpDownSpeedMultiplier
  (params (ClimbUpSpeedMuliplier :type Float%20%28single-precision%29) (ClimbDownSpeedMuliplier :type Float%20%28single-precision%29)))

(fn RopeClimbingActivated/Deactivated
  (params (Activated/Deactivated :type Boolean)))

(fn RopeClimbingMovementState
  (params (State :type Byte)))

(fn RopeClimbingPhysicsActivated/Deactivated
  (params (Activated/Deactivated :type Boolean)))

(fn RopeClimbOverlayResponse
  (params (Disable :type Boolean)))

(fn DisableRopeGrab
  (return false))

(fn SwingingInputs
  (return 0.0 0.0))

(fn RopeClimbOverlay
  (return false 0 false))

(fn RopeFinishExt
  (return false))

(fn RopeStartExt
  (params (Index :type Integer) (HorizontalMovement :type Boolean) (PreDelay :type Float%20%28single-precision%29) (MovementTime :type Float%20%28single-precision%29))
  (return false))

(fn RopeGobalCollect
  (params (SearchLocation :type Vector) (Radius :type Float%20%28single-precision%29))
  (return false))

(fn RopeClimbingAutoMovement
  (params (bAutoMovement :type Boolean)))