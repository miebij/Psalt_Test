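; Blueprint interface for the pole climbing camera in the Advanced Traversal System.
; It declares calls to pass in the character, player camera and controller references, and to update climb state flags such as on top, aiming, turning and climbing up or down.
; Further calls update camera data, alpha, rotation, offset and FOV, and add, remove or reset the camera, with blend times for adding and removing.
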(fn SetPoleClimbCameraCharRef
  (params (Character :type Actor%20Object%20Reference) (PlayerCamera :type Player%20Camera%20Manager%20Object%20Reference) (PlayerController :type Player%20Controller%20Object%20Reference))
  (return false))

(fn UpdatePoleClimbCameraState
  (params (MoveTo :type Boolean) (OnTop :type Boolean) (Aiming :type Boolean) (Turning :type Boolean) (ClimbUp :type Boolean) (ClimbDown :type Boolean))
  (return false))

(fn UpdatePoleClimbCameraDatas
  (return false))

(fn UpdatePoleClimbAlpha
  (params (Alpha :type Float%20%28double-precision%29))
  (return false))

(fn UpdatePoleClimbCameraRotation
  (params (TargetRotation :type Rotator))
  (return false))

(fn UpdatePoleClimbCameraOffset
  (params (Offset :type Vector))
  (return false))

(fn UpdatePoleClimbCameraFOV
  (params (FOV :type Float%20%28double-precision%29))
  (return false))

(fn AddPoleClimbCamera
  (params (BlendInTime :type Float%20%28double-precision%29))
  (return false))

(fn RemovePoleClimbCamera
  (params (BlendOutTime :type Float%20%28double-precision%29))
  (return false))

(fn ResetPoleClimbCamera
  (return false))