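; LadderClimbing_BPI is the Blueprint Interface for the ladder climbing part of the Advanced Traversal System.
; Its messages carry climb states such as grab, jump, reach, slide and release, plus player and AI input, speed, and hand and foot placement.
; Others relay per-limb anim notifies, system and physics toggles, camera switching and aiming overlays.
; Functions with return values cover grab blocking, input and overlay queries, external start/finish and radius-based ladder collection.
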(fn GrabLadderStates
  (params (Grab_Ladder :type Boolean) (GrabFromAir :type Boolean) (H-Angle :type Float%20%28single-precision%29) (GrabState :type Integer)))

(fn LadderSide
  (params (Right? :type Boolean)))

(fn LadderClimbUp
  (params (Climb_Up_Ladder :type Boolean)))

(fn Jump/ClimbtoLadder
  (params (Jump_To_Ladder :type Boolean) (Climb_To_Laddder :type Boolean) (Climb/JumpBackward :type Boolean) (Distance :type Float%20%28single-precision%29) (Angle :type Float%20%28single-precision%29) (Side :type Float%20%28single-precision%29)))

(fn LadderMovementDirection
  (params (Upward? :type Boolean)))

(fn ReleaseLadder
  (params (Release_Ladder :type Boolean)))

(fn EnableLadderSystem
  (params (Enable_System :type Boolean) (BlendIn :type Float%20%28single-precision%29) (BlendOut :type Float%20%28single-precision%29)))

(fn FreeJump
  (params (FreeJumping :type Boolean) (JumpBackward :type Boolean) (FreeJumpAngle :type Float%20%28single-precision%29) (FreeJumpSide :type Float%20%28single-precision%29) (FreeJumpVelocity :type Float%20%28single-precision%29)))

(fn LadderInput
  (params (Move_Forward_Ladder :type Float%20%28single-precision%29) (Move_Right_Ladder :type Float%20%28single-precision%29)))

(fn AIInput
  (params (Ground/Top :type Boolean) (AiMoveForward :type Float%20%28single-precision%29)))

(fn LadderClimbingSpeed
  (params (ClimbingSpeed :type Float%20%28single-precision%29)))

(fn LadderMovementAlpha
  (params (Ladder_Movement_Alpha :type Float%20%28single-precision%29)))

(fn CurrentHandLocation
  (params (Hand_R :type Vector) (Rot_R :type Rotator) (Hand_L :type Vector) (Rot_L :type Rotator)))

(fn NewHandLocation
  (params (Hand_R :type Vector) (Rot_R :type Rotator) (Hand_L :type Vector) (Rot_L :type Rotator)))

(fn CurrentFootLocation
  (params (Foot_R :type Vector) (Foot_L :type Vector)))

(fn NewFootLocation
  (params (Foot_R :type Vector) (Foot_L :type Vector)))

(fn AnimNotifyLadderHandR)

(fn AnimNotifyLadderHandL)

(fn AnimNotifyLadderFootR)

(fn AnimNotifyLadderFootL)

(fn LadderClimbingSystemActivated/Deactived
  (params (Activated/Deactived :type Boolean)))

(fn LadderPhysicsActivated/Deactivated
  (params (Activated/Deactivated :type Boolean)))

(fn LadderClimbingMovementStates
  (params (State :type Byte)))

(fn LadderClimbOverlayResponse
  (params (Disable :type Boolean)))

(fn LadderSwitchCamera
  (params (Right :type Boolean)))

(fn DisableLadderGrab
  (return false))

(fn LadderClimbingInputs
  (return 0.0 0.0))

(fn LadderClimbOverlay
  (return false 0 false))

(fn LadderFinishExt
  (return false))

(fn LadderStartExt
  (params (Index :type Integer) (HorizontalMovement :type Boolean) (PreDelay :type Float%20%28single-precision%29) (MovementTime :type Float%20%28single-precision%29))
  (return false))

(fn LadderGobalCollect
  (params (SearchLocation :type Vector) (Radius :type Float%20%28single-precision%29))
  (return false))

(fn LadderExternal
  (params (ClimbingExternalIn :type Boolean) (ClimbingExternalOut :type Boolean) (AngleExt :type Float%20%28single-precision%29) (SideExt :type Float%20%28single-precision%29) (DistanceExt :type Float%20%28single-precision%29)))

(fn LadderReach
  (params (Reach :type Boolean) (ReachBackward :type Boolean) (ReachForward :type Float%20%28single-precision%29) (ReachRight :type Float%20%28single-precision%29)))

(fn SlideDown
  (params (SlidingDown :type Boolean) (SlidingDownStart :type Boolean) (SlidingDownEnd :type Boolean)))

(fn LadderClimbAimingStates
  (params (UseOverlay :type Boolean) (Aiming :type Boolean) (Ready :type Boolean) (Stand :type Boolean) (AimingRotation :type Rotator)))