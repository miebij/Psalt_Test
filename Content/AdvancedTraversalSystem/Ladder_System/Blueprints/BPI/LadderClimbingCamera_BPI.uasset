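; Blueprint interface through which the ladder climbing system of an advanced traversal setup drives its climbing camera.
; It passes in character, camera and controller references, then updates climb state flags for moving, sliding down, turning back and aiming.
; Further calls update the climb alpha, target rotation, offset, FOV and camera data.
; Add, remove and reset functions control the camera, with blend times for entering and leaving.
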(fn SetLadderClimbCameraCharRef
  (params (Character :type Actor%20Object%20Reference) (PlayerCamera :type Player%20Camera%20Manager%20Object%20Reference) (PlayerController :type Player%20Controller%20Object%20Reference))
  (return false))

(fn UpdateLadderClimbCameraState
  (params (MoveTo :type Boolean) (SlideDown :type Boolean) (TurnBack :type Boolean) (Aiming :type Boolean))
  (return false))

(fn UpdateLadderClimbCameraDatas
  (return false))

(fn UpdateLadderClimbAlpha
  (params (Alpha :type Float%20%28double-precision%29))
  (return false))

(fn UpdateLadderClimbCameraRotation
  (params (TargetRotation :type Rotator))
  (return false))

(fn UpdateLadderClimbCameraOffset
  (params (Offset :type Vector))
  (return false))

(fn UpdateLadderClimbCameraFOV
  (params (FOV :type Float%20%28double-precision%29))
  (return false))

(fn AddLadderClimbingCamera
  (params (BlendInTime :type Float%20%28double-precision%29))
  (return false))

(fn RemoveLadderClimbingCamera
  (params (BlendOutTime :type Float%20%28double-precision%29))
  (return false))

(fn ResetLadderClimbingCamera
  (return false))