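; Sound function collection for the ladder climbing system, playing hand, foot and jump audio.
; Hand and foot functions pick a metal, wood or default sound from the hit's surface type, playing it at the impact point facing into the surface.
; The jump function plays at the target component's transform.
; The sliding function is empty, with its attached metal-slide spawn and stop logic left unconnected.
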(fn LadderHandSounds
  (params (Hit :type Hit%20Result%20Structure%20%28by%20ref%29))
  (bind (_bblockinghit _binitialoverlap _time _distance _location _impactpoint _normal _impactnormal) (Collision|BreakHitResult Hit))
  ;[0.1062 0.2344 0.1482 1 100] Hand Sounds
  (LocalVariables|SetLocation _impactpoint)
  (LocalVariables|SetRotation (Math|Rotator|MakeRotfromX (* _impactnormal -1)))
  (switch Utilities|FlowControl|Switch|SwitchonEPhysicalSurface (Collision|GetSurfaceType Hit)
    (:SurfaceType_Default
      (Audio|PlaySoundatLocation 0 (LocalVariables|GetLadderHandDefaultSound) (LocalVariables|GetLocation) (LocalVariables|GetRotation) 5.0 1.0 0.0 0 0 0 0))
    (:SurfaceType5
      (Audio|PlaySoundatLocation 0 (LocalVariables|GetLadderHandMetalSound) (LocalVariables|GetLocation) (LocalVariables|GetRotation) 7.0 1.0 0.0 0 0 0 0))
    (:SurfaceType6
      (Audio|PlaySoundatLocation 0 (LocalVariables|GetLadderWoodSound) (LocalVariables|GetLocation) (LocalVariables|GetRotation) 2.0 1.0 0.0 0 0 0 0))))

(fn LadderFootSounds
  (params (Hit :type Hit%20Result%20Structure%20%28by%20ref%29))
  (bind (_bblockinghit _binitialoverlap _time _distance _location _impactpoint _normal _impactnormal) (Collision|BreakHitResult Hit))
  ;[0.2344 0.1036 0.08959 1 100] Foot Sounds
  (LocalVariables|SetLocation _impactpoint)
  (LocalVariables|SetRotation (Math|Rotator|MakeRotfromX (* _impactnormal -1)))
  (switch Utilities|FlowControl|Switch|SwitchonEPhysicalSurface (Collision|GetSurfaceType Hit)
    (:SurfaceType_Default
      (Audio|PlaySoundatLocation 0 (LocalVariables|GetLadderDefaultSound) (LocalVariables|GetLocation) (LocalVariables|GetRotation) 5.0 1.0 0.0 0 0 0 0))
    (:SurfaceType5
      (Audio|PlaySoundatLocation 0 (LocalVariables|GetLadderMetalFootSound) (LocalVariables|GetLocation) (LocalVariables|GetRotation) 7.0 1.0 0.0 0 0 0 0))
    (:SurfaceType6
      (Audio|PlaySoundatLocation 0 (LocalVariables|GetLadderWoodSound) (LocalVariables|GetLocation) (LocalVariables|GetRotation) 3.0 1.0 0.0 0 0 0 0))))

(fn LadderJumpSound
  (params (Target :type Scene%20Component%20Object%20Reference))
  (Audio|PlaySoundatLocation 0 (LocalVariables|GetJumpSound) (Transformation|GetWorldLocation Target) (Transformation|GetWorldRotation Target) 1.8 1.0 0.0 0 0 0 0))

(fn LadderSliding
  (params (AttachToComponent :type Scene%20Component%20Object%20Reference) (Add :type Boolean) (Target :type Audio%20Component%20Object%20Reference)))