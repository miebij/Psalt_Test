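; Function library for the wall climbing system that spawns impact particles for axe, hand and foot contacts.
; Each function takes a hit result, places a pooled, auto-released effect at the impact point and orients it along the inverted impact normal.
; The hit's surface type selects the effect: Ice gets its own variant, while Ground, Rock, Foliage and any other surface share the ground effect.
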(fn WallAxeParticles
  (params (Hit :type Hit%20Result%20Structure%20%28by%20ref%29))
  (bind (_bblockinghit _binitialoverlap _time _distance _location _impactpoint _normal _impactnormal) (Collision|BreakHitResult Hit))
  ;[0.1823 0.1196 0.09752 1 100] Axe Particles
  (LocalVariables|SetLocation _impactpoint)
  (LocalVariables|SetRotation (Math|Rotator|MakeRotfromX (* _impactnormal -1)))
  (switch Utilities|FlowControl|Switch|SwitchonEPhysicalSurface (Collision|GetSurfaceType Hit)
    (:SurfaceType_Default
      (Niagara|SpawnSystematLocation 0 (LocalVariables|GetAxeGroundHit) (LocalVariables|GetLocation) (LocalVariables|GetRotation) "1.000000,1.000000,1.000000" true true "AutoRelease"))
    (:SurfaceType1
      (Niagara|SpawnSystematLocation 0 (LocalVariables|GetAxeIceHit) (LocalVariables|GetLocation) (LocalVariables|GetRotation) "1.000000,1.000000,1.000000" true true "AutoRelease"))
    (:SurfaceType2
      (Niagara|SpawnSystematLocation 0 (LocalVariables|GetAxeGroundHit) (LocalVariables|GetLocation) (LocalVariables|GetRotation) "1.000000,1.000000,1.000000" true true "AutoRelease" :!label _label))
    (:SurfaceType3
      (goto _label))
    (:SurfaceType4
      (goto _label))))

(fn WallHandParticles
  (params (Hit :type Hit%20Result%20Structure%20%28by%20ref%29))
  (bind (_bblockinghit _binitialoverlap _time _distance _location _impactpoint _normal _impactnormal) (Collision|BreakHitResult Hit))
  ;[0.2344 0.2261 0.1416 1 100] Hand Particles
  (LocalVariables|SetLocation _impactpoint)
  (LocalVariables|SetRotation (Math|Rotator|MakeRotfromX (* _impactnormal -1)))
  (switch Utilities|FlowControl|Switch|SwitchonEPhysicalSurface (Collision|GetSurfaceType Hit)
    (:SurfaceType_Default
      (Niagara|SpawnSystematLocation 0 (LocalVariables|GetHandGroundDust) (LocalVariables|GetLocation) (LocalVariables|GetRotation) "1.000000,1.000000,1.000000" true true "AutoRelease"))
    (:SurfaceType1
      (Niagara|SpawnSystematLocation 0 (LocalVariables|GetHandIceDust) (LocalVariables|GetLocation) (LocalVariables|GetRotation) "1.000000,1.000000,1.000000" true true "AutoRelease"))
    (:SurfaceType2
      (Niagara|SpawnSystematLocation 0 (LocalVariables|GetHandGroundDust) (LocalVariables|GetLocation) (LocalVariables|GetRotation) "1.000000,1.000000,1.000000" true true "AutoRelease" :!label _label))
    (:SurfaceType3
      (goto _label))
    (:SurfaceType4
      (goto _label))))

(fn WallFootParticles
  (params (Hit :type Hit%20Result%20Structure%20%28by%20ref%29))
  (bind (_bblockinghit _binitialoverlap _time _distance _location _impactpoint _normal _impactnormal) (Collision|BreakHitResult Hit))
  ;[0.09766 0.2344 0.2344 1 100] Foot Particles
  (LocalVariables|SetLocation _impactpoint)
  (LocalVariables|SetRotation (Math|Rotator|MakeRotfromX (* _impactnormal -1)))
  (switch Utilities|FlowControl|Switch|SwitchonEPhysicalSurface (Collision|GetSurfaceType Hit)
    (:SurfaceType_Default
      (Niagara|SpawnSystematLocation 0 (LocalVariables|GetFootGroundDust) (LocalVariables|GetLocation) (LocalVariables|GetRotation) "1.000000,1.000000,1.000000" true true "AutoRelease"))
    (:SurfaceType1
      (Niagara|SpawnSystematLocation 0 (LocalVariables|GetFootIceDust) (LocalVariables|GetLocation) (LocalVariables|GetRotation) "1.000000,1.000000,1.000000" true true "AutoRelease"))
    (:SurfaceType2
      (Niagara|SpawnSystematLocation 0 (LocalVariables|GetFootGroundDust) (LocalVariables|GetLocation) (LocalVariables|GetRotation) "1.000000,1.000000,1.000000" true true "AutoRelease" :!label _label))
    (:SurfaceType3
      (goto _label))
    (:SurfaceType4
      (goto _label))))