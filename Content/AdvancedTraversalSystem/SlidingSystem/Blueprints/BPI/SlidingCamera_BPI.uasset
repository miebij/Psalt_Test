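; Blueprint interface for the camera used by the sliding part of the Advanced Traversal System.
; It declares calls to pass in character, camera and controller references, and to update aiming state, camera data and slide alpha.
; Further calls set rotation, offset and FOV, and add, remove or reset the sliding camera with timed blend in and out.
; It holds only signatures, leaving behavior to implementers.
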(fn SetSlidingCameraCharRef
  (params (Character :type Actor%20Object%20Reference) (PlayerCamera :type Player%20Camera%20Manager%20Object%20Reference) (PlayerController :type Player%20Controller%20Object%20Reference))
  (return false))

(fn UpdateSlidingCameraState
  (params (Aiming :type Boolean))
  (return false))

(fn UpdateSlidingCameraDatas
  (return false))

(fn UpdateSlidingAlpha
  (params (Alpha :type Float%20%28single-precision%29))
  (return false))

(fn UpdateSlidingCameraRotation
  (params (TargetRotation :type Rotator))
  (return false))

(fn UpdateSlidingCameraOffset
  (params (Offset :type Vector))
  (return false))

(fn UpdateSlidingCameraFOV
  (params (FOV :type Float%20%28single-precision%29))
  (return false))

(fn AddSlidingCamera
  (params (BlendInTime :type Float%20%28single-precision%29))
  (return false))

(fn RemoveSlidingCamera
  (params (BlendOutTime :type Float%20%28single-precision%29))
  (return false))

(fn ResetSlidingCamera
  (return false))