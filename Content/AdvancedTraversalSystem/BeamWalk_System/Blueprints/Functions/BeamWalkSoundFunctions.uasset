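; Sound function collection for the beam walk traversal system, playing footstep and jump audio.
; The footstep function switches on the hit's surface type and plays at the impact point, oriented against the surface normal.
; Only Wood and Concrete differ from the default sound, and their sound assets are crossed: Wood plays the concrete sound, Concrete the wood one.
; The jump function plays one sound at the target's world transform.
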(fn BeamWalkFootSounds
  (params (Hit :type Hit%20Result%20Structure%20%28by%20ref%29))
  (bind (_bblockinghit _binitialoverlap _time _distance _location _impactpoint _normal _impactnormal) (Collision|BreakHitResult Hit))
  ;[0.2344 0.1036 0.08959 1 100] Foot Sounds
  (LocalVariables|SetLocation _impactpoint)
  (LocalVariables|SetRotation (Math|Rotator|MakeRotfromX (* _impactnormal -1)))
  (switch Utilities|FlowControl|Switch|SwitchonEPhysicalSurface (Collision|GetSurfaceType Hit)
    (:SurfaceType_Default
      (Audio|PlaySoundatLocation 0 (LocalVariables|GetBeamWalkDefaultSound) (LocalVariables|GetLocation) (LocalVariables|GetRotation) 1.5 1.0 0.0 0 0 0 0 :!label _label))
    (:SurfaceType1
      (goto _label))
    (:SurfaceType2
      (goto _label))
    (:SurfaceType3
      (goto _label))
    (:SurfaceType4
      (goto _label))
    (:SurfaceType5
      (goto _label))
    (:SurfaceType6
      (Audio|PlaySoundatLocation 0 (LocalVariables|GetBeamWalkConcreteSound) (LocalVariables|GetLocation) (LocalVariables|GetRotation) 1.0 1.0 0.0 0 0 0 0))
    (:SurfaceType7
      (goto _label))
    (:SurfaceType8
      (goto _label))
    (:SurfaceType9
      (Audio|PlaySoundatLocation 0 (LocalVariables|GetBeamWalkWoodSound) (LocalVariables|GetLocation) (LocalVariables|GetRotation) 1.5 1.0 0.0 0 0 0 0) ; Foliage
    )))

(fn BeamWalkJumpSound
  (params (Target :type Scene%20Component%20Object%20Reference))
  (Audio|PlaySoundatLocation 0 (LocalVariables|GetJumpSound) (Transformation|GetWorldLocation Target) (Transformation|GetWorldRotation Target) 1.2 1.0 0.0 0 0 0 0))