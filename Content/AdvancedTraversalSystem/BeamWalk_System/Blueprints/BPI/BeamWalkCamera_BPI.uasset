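; Blueprint Interface for the camera of the beam walk system in an advanced traversal setup.
; It declares calls to pass character, camera and controller references, update camera state from move, balance and aiming inputs, and refresh camera data.
; Further calls drive alpha, rotation, offset and FOV, and add, remove or reset the camera, with blend times for adding and removing.
; It holds only signatures, leaving behavior to implementers.
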(fn SetBeamWalkCameraCharRef
  (params (Character :type Actor%20Object%20Reference) (PlayerCamera :type Player%20Camera%20Manager%20Object%20Reference) (PlayerController :type Player%20Controller%20Object%20Reference))
  (return false))

(fn UpdateBeamWalkCameraState
  (params (MoveTo :type Boolean) (Balance :type Boolean) (Aiming :type Boolean))
  (return false))

(fn UpdateBeamWalkCameraDatas
  (return false))

(fn UpdateBeamWalkAlpha
  (params (Alpha :type Float%20%28double-precision%29))
  (return false))

(fn UpdateBeamWalkCameraRotation
  (params (TargetRotation :type Rotator))
  (return false))

(fn UpdateBeamWalkCameraOffset
  (params (Offset :type Vector))
  (return false))

(fn UpdateBeamWalkCameraFOV
  (params (FOV :type Float%20%28double-precision%29))
  (return false))

(fn AddBeamWalkCamera
  (params (BlendInTime :type Float%20%28double-precision%29))
  (return false))

(fn RemoveBeamWalkCamera
  (params (BlendOutTime :type Float%20%28double-precision%29))
  (return false))

(fn ResetBeamWalkCamera
  (return false))