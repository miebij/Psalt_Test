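; Anim notify for the beam walk traversal system that triggers footstep or jump sounds from animations.
; In Foot mode it line-traces vertically on the Visibility channel around the mesh's root socket, ignoring the owner, and passes any hit to BeamWalkFootSounds.
; In Jump mode it calls BeamWalkJumpSound with the mesh, without tracing.
; The notify's displayed name follows the active flag, with Foot taking priority over Jump.
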(fn ReceivedNotify
  (params (MeshComp :type Skeletal%20Mesh%20Component%20Object%20Reference) (Animation :type Anim%20Sequence%20Base%20Object%20Reference) (EventReference :type Anim%20Notify%20Event%20Reference%20Structure%20%28by%20ref%29))
  (bind _returnvalue (Transformation|GetSocketLocation MeshComp "root"))
  (if (Variables|Default|GetFoot)
    (bind (_outhit _returnvalue_2) (Collision|LineTraceByChannel (+ _returnvalue "0, 0,40.000000") (- _returnvalue "0, 0,40.000000") "TraceTypeQuery1" false (Utilities|Array|MakeArray (Components|GetOwner MeshComp)) "None"))
    (if _returnvalue_2
      (CallFunction|BeamWalkFootSounds _outhit)
      (return true)
      (else
        (return false)))
    (elif (Variables|Default|GetJump)
      (CallFunction|BeamWalkJumpSound MeshComp))))

(fn GetNotifyName
  (if (Variables|Default|GetFoot)
    (return "Foot")
    (elif (Variables|Default|GetJump)
      (return "Jump")
      (else
        (return "None")))))