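; Camera modifier for the swimming system that offsets the player camera and blends its location and FOV in and out.
; A three-state machine handles enter, movement and exit, removing the modifier once blend-out completes.
; Movement picks surface, underwater, dive transition or interaction placement relative to water level, easing toward the character when close.
; A sphere trace pulls the camera in on collisions, and setter functions supply state, offsets, FOV and water level.
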(fn BlueprintModifyCamera
  (params (DeltaTime :type Float%20%28single-precision%29) (ViewLocation :type Vector :default "0, 0, 0") (ViewRotation :type Rotator :default "0, 0, 0") (FOV :type Float%20%28single-precision%29))
  (bind _targetfov (Variables|Default|GetTargetFOV))
  (bind _cameralocation (CallFunction|GetCameraLocation ViewLocation ViewRotation))
  (bind _cameralocation_2 (CallFunction|GetCameraLocation ViewLocation ViewRotation))
  (bind (_newlocation _newrotation) (Handles|Interaction ViewLocation ViewRotation))
  (bind (_newlocation_2 _returnvalue) (Handles|Dive2Swim _cameralocation_2 ViewRotation DeltaTime))
  (bind (_newlocation_3 _returnvalue_2) (Handles|Swim2Dive _cameralocation ViewLocation ViewRotation DeltaTime))
  (|UpdateOffset)
  (Collision|CameraCorrection ViewLocation)
  (switch int (Variables|Default|GetState)
    (:0
      ;[0.1594 0.4792 0.1817] Enter
      (Variables|Blend|SetBlendIn_cnt (+ (Variables|Blend|GetBlendIn_cnt) DeltaTime))
      (Variables|Blend|SetBlendOut_cnt 0.0)
      (if (|BlendIn)
        (Variables|Default|SetState 1))
      (Pawn|SetControlRotation (Variables|References|GetPlayer%20Controller) ViewRotation)
      (return (Math|Vector|Lerp(Vector) ViewLocation (CallFunction|GetCameraLocation ViewLocation ViewRotation) (Blends|BlendinAlpha)) ViewRotation (Math|Float|Lerp (Camera|GetFOVAngle (Variables|CameraModifier|GetCameraOwner)) (Variables|Default|GetTargetFOV) (Blends|BlendinAlpha))))
    (:1
      ;[0.04312 0.3633 0.4792] Movement
      (if (Variables|States|GetInteract)
        (Pawn|SetControlRotation (Variables|References|GetPlayer%20Controller) _newrotation)
        (return _newlocation ViewRotation (Variables|Default|GetTargetFOV))
        (elif (Variables|States|GetDive%202Swim)
          (Pawn|SetControlRotation (Variables|References|GetPlayer%20Controller) _returnvalue)
          ;[0.04312 0.3633 0.4792] Movement
          (return _newlocation_2 _returnvalue (Variables|Default|GetTargetFOV))
          (elif (Variables|States|GetSwim%202Dive)
            (Pawn|SetControlRotation (Variables|References|GetPlayer%20Controller) _returnvalue_2)
            (return _newlocation_3 _returnvalue_2 (Variables|Default|GetTargetFOV))
            (elif (Variables|States|GetDive)
              (Pawn|SetControlRotation (Variables|References|GetPlayer%20Controller) ViewRotation)
              (return (Handles|SwimUnderwater (CallFunction|GetCameraLocation ViewLocation ViewRotation) ViewLocation) ViewRotation (Math|Interpolation|FInterpTo _targetfov _targetfov DeltaTime 5.0))
              (else
                (Pawn|SetControlRotation (Variables|References|GetPlayer%20Controller) ViewRotation)
                (return (Handles|SwimSurface (CallFunction|GetCameraLocation ViewLocation ViewRotation)) ViewRotation (Variables|Default|GetTargetFOV))))))))
    (:2
      ;[0.4792 0.1848 0.1417] Exit
      (Variables|Blend|SetBlendOut_cnt (+ (Variables|Blend|GetBlendOut_cnt) DeltaTime))
      (Variables|Blend|SetBlendIn_cnt 0.0)
      (if (|BlendOut)
        (Game|Player|RemoveCameraModifier (Variables|References|GetPlayerCamera) self)
        (else
          (return (Math|Vector|Lerp(Vector) (Camera|GetCameraLocation (Variables|CameraModifier|GetCameraOwner)) ViewLocation (Blends|BlendOutAlpha)) (Misc|RemoveRoll (Math|Rotator|Lerp(Rotator) (Camera|GetCameraRotation (Variables|CameraModifier|GetCameraOwner)) ViewRotation (Blends|BlendOutAlpha) true)) (Math|Float|Lerp (Camera|GetFOVAngle (Variables|CameraModifier|GetCameraOwner)) FOV (Blends|BlendOutAlpha))))))))

(fn GetCameraLocation
  (params (ViewLocation :type Vector) (ViewRotation :type Rotator))
  (bind _offset (Variables|Default|GetOffset))
  (bind _characteractor (Variables|References|GetCharacterActor))
  (bind (_x _y _z) (Math|Vector|BreakVector _offset))
  (return (+ ViewLocation (* (Transformation|GetActorRightVector _characteractor) _x) (* (Math|Vector|GetForwardVector ViewRotation) (+ _y (.Y (Math|Vector|BreakVector (Variables|Default|GetCorrection))))) (* (Transformation|GetActorUpVector _characteractor) _z))))

(fn CameraCorrection
  (params (ViewLocation :type Vector))
  (bind (_start _end) (|CameraTraceParams ViewLocation))
  ;[0.4219 0.3478 0.173] Camera Correction
  (bind (_outhit _returnvalue) (Collision|CollisionTrace _start _end))
  (if _returnvalue
    (if (.Yes (|NeedToCorrect (.Location (Collision|BreakHitResult _outhit)) (.TraceStart (Collision|BreakHitResult _outhit)) ViewLocation))
      (Variables|Default|SetCorrection (Math|Vector|MakeVector 0.0 (.CorrectionValue (|NeedToCorrect (.Location (Collision|BreakHitResult _outhit)) (.TraceStart (Collision|BreakHitResult _outhit)) ViewLocation)) 0.0))
      (else
        (Variables|Default|SetCorrection "0, 0, 0" :!label _label)))
    (else
      (goto _label))))

(fn CollisionTrace
  (params (Start :type Vector) (End :type Vector))
  (if (or (Variables|States|GetDive%202Swim) (Variables|States|GetSwim%202Dive))
    (bind _outhit (Collision|SphereTraceByChannel Start End 2e+01 "TraceTypeQuery1" false (Utilities|Array|MakeArray (Variables|References|GetCharacterActor)) "None")) ; Overlap water plane
    (return _outhit (and (.bBlockingHit (Collision|BreakHitResult _outhit)) (not (.bInitialOverlap (Collision|BreakHitResult _outhit)))))
    (else
      (bind (_outhit_2 _returnvalue) (Collision|SphereTraceForObjects Start End 2e+01 (Utilities|Array|MakeArray "ObjectTypeQuery1") false (Utilities|Array|MakeArray (Variables|References|GetCharacterActor)) "None")) ; Colliside with water plane
      (return _outhit_2 _returnvalue))))

(fn BlendinAlpha
  (return (Math|Float|Clamp(Float) (/ (Variables|Blend|GetBlendIn_cnt) (Variables|Blend|GetBlendInTime)))))

(fn BlendOutAlpha
  (return (Math|Float|Clamp(Float) (/ (Variables|Blend|GetBlendOut_cnt) (Variables|Blend|GetBlendOutTime)))))

(fn RemoveRoll
  (params (Rotation :type Rotator))
  (bind (_roll _pitch _yaw) (Math|Rotator|BreakRotator Rotation))
  (return (Math|Rotator|MakeRotator 0.0 _pitch _yaw)))

(fn SwimSurface
  (params (Location+Offset :type Vector))
  (bind _characteractor (Variables|References|GetCharacterActor))
  (bind _characteractor_2 (Variables|References|GetCharacterActor))
  (bind (_x _y) (Math|Vector|BreakVector Location+Offset))
  (bind _returnvalue (Transformation|GetActorLocation _characteractor_2))
  (bind _returnvalue_2 (Transformation|GetActorLocation _characteractor))
  (bind (_x_2 _y_2) (Math|Vector|BreakVector _returnvalue))
  (bind (_x_3 _y_3) (Math|Vector|BreakVector _returnvalue_2))
  (if (>= (.Z (Math|Vector|BreakVector (Transformation|GetActorForwardVector (Variables|References|GetPlayerCamera)))) 0.0)
    (LocalVariables|SetDistance-Local (Math|Vector|VectorLength (- (Math|Vector|MakeVector _x _y 0.0) (Math|Vector|MakeVector _x_3 _y_3 0.0))))
    (else
      (LocalVariables|SetDistance-Local (Math|Vector|VectorLength (- Location+Offset (Transformation|GetActorLocation (Variables|References|GetCharacterActor)))))))
  (if (<= (LocalVariables|GetDistance-Local) 1.5e+02)
    (return (Math|Vector|Lerp(Vector) (Math|Vector|SelectVector Location+Offset Location+Offset (<= (.Z (Math|Vector|BreakVector Location+Offset)) (+ (Variables|Default|GetWaterLevel) 2e+01))) (Math|Vector|MakeVector _x_2 _y_2 (+ (Variables|Default|GetWaterLevel) 1e+02)) (Math|Float|MapRangeClamped (LocalVariables|GetDistance-Local) 1.5e+02 0.0 0.0 1.0)))
    (else
      (return (Math|Vector|SelectVector Location+Offset Location+Offset (<= (.Z (Math|Vector|BreakVector Location+Offset)) (+ (Variables|Default|GetWaterLevel) 2e+01)))))))

(fn SwimUnderwater
  (params (Location+Offset :type Vector) (ViewLocationIn :type Vector))
  (bind _characteractor (Variables|References|GetCharacterActor))
  (bind _returnvalue (Transformation|GetActorLocation _characteractor))
  (LocalVariables|SetDistance-Local (Math|Vector|VectorLength (- Location+Offset (Transformation|GetActorLocation (Variables|References|GetCharacterActor)))))
  (if (<= (LocalVariables|GetDistance-Local) 1.5e+02)
    (return (Math|Vector|Lerp(Vector) (Math|Vector|SelectVector Location+Offset Location+Offset (>= (.Z (Math|Vector|BreakVector Location+Offset)) (+ (Variables|Default|GetWaterLevel) -2e+01))) (+ _returnvalue (* (Math|Vector|Normalize (- ViewLocationIn _returnvalue)) 8e+01) "0,0,40.000000") (Math|Float|MapRangeClamped (LocalVariables|GetDistance-Local) 1.5e+02 0.0 0.0 1.0)))
    (else
      (return (Math|Vector|SelectVector Location+Offset Location+Offset (>= (.Z (Math|Vector|BreakVector Location+Offset)) (+ (Variables|Default|GetWaterLevel) -2e+01)))))))

(fn Dive2Swim
  (params (Location+Offset :type Vector) (ViewRotationIn :type Rotator) (DeltaTime :type Float%20%28single-precision%29))
  (return (Math|Interpolation|VInterpTo Location+Offset (Handles|SwimSurface Location+Offset) DeltaTime 1e+01) (Math|Interpolation|RInterpTo ViewRotationIn (Math|Rotator|MakeRotator 0.0 -1e+01 (.Yaw (Math|Rotator|BreakRotator ViewRotationIn))) DeltaTime 1e+01)))

(fn Swim2Dive
  (params (Location+Offset :type Vector) (ViewLocationIn :type Vector) (ViewRotationIn :type Rotator) (DeltaTime :type Float%20%28single-precision%29))
  (return (Math|Interpolation|VInterpTo (Camera|GetCameraLocation (Variables|References|GetPlayerCamera)) (Handles|SwimUnderwater Location+Offset ViewLocationIn) DeltaTime 4e+01) (Math|Interpolation|RInterpTo (Camera|GetCameraRotation (Variables|References|GetPlayerCamera)) ViewRotationIn DeltaTime 4e+01)))

(fn Interaction
  (params (ViewLocationIn :type Vector) (ViewRotationIn :type Rotator))
  (if (Variables|States|GetDive)
    (return (Math|Interpolation|VInterpTo (Handles|SwimUnderwater (CallFunction|GetCameraLocation ViewLocationIn ViewRotationIn) ViewLocationIn) (Handles|SwimUnderwater (CallFunction|GetCameraLocation ViewLocationIn (Transformation|GetActorRotation (Variables|References|GetCharacterActor))) ViewLocationIn) (Utilities|Time|GetWorldDeltaSeconds) 5.0) (Math|Interpolation|RInterpTo ViewRotationIn (Transformation|GetActorRotation (Variables|References|GetCharacterActor)) (Utilities|Time|GetWorldDeltaSeconds) 5.0))
    (else
      (return (Math|Interpolation|VInterpTo (Handles|SwimSurface (CallFunction|GetCameraLocation ViewLocationIn ViewRotationIn)) (Handles|SwimSurface (CallFunction|GetCameraLocation ViewLocationIn (Transformation|GetActorRotation (Variables|References|GetCharacterActor)))) (Utilities|Time|GetWorldDeltaSeconds) 5.0) (Math|Interpolation|RInterpTo ViewRotationIn (Transformation|GetActorRotation (Variables|References|GetCharacterActor)) (Utilities|Time|GetWorldDeltaSeconds) 5.0)))))

(fn AddSwimmingCamera
  (params (BlendInTime :type Float%20%28single-precision%29))
  (Variables|Blend|SetBlendInTime BlendInTime)
  (Variables|Default|SetState 0)
  (return true))

(fn RemoveSwimmingCamera
  (params (BlendOutTime :type Float%20%28single-precision%29))
  (Variables|Blend|SetBlendOutTime BlendOutTime)
  (Variables|Default|SetState 2)
  (return true))

(fn ResetSwimmingCamera
  (Variables|Default|SetState 0)
  (return true))

(fn SetSwimCameraCharRef
  (params (Character :type Actor%20Object%20Reference) (PlayerCamera :type Player%20Camera%20Manager%20Object%20Reference) (PlayerController :type Player%20Controller%20Object%20Reference))
  (Variables|References|SetCharacterActor Character)
  (Variables|References|SetPlayerCamera PlayerCamera)
  (Variables|References|SetPlayer%20Controller PlayerController)
  (return true))

(fn UpdateSwimAlpha
  (params (Alpha :type Float%20%28single-precision%29))
  (return false))

(fn UpdateSwimCameraDatas
  (params (WaterLevel :type Float%20%28single-precision%29))
  (Variables|Default|SetWaterLevel WaterLevel)
  (return true))

(fn UpdateSwimCameraFOV
  (params (FOV :type Float%20%28single-precision%29))
  (Variables|Default|SetTargetFOV FOV)
  (return true))

(fn UpdateSwimCameraOffset
  (params (OffsetSwim :type Vector :default "0, 0, 0") (OffsetFastSwim :type Vector :default "0, 0, 0"))
  (Variables|Default|SetOffsetSwim OffsetSwim)
  (Variables|Default|SetOffsetFastSwim OffsetFastSwim)
  (return true))

(fn UpdateSwimCameraRotation
  (params (TargetRotation :type Rotator :default "0, 0, 0"))
  (Variables|Default|SetTargetRotation TargetRotation)
  (return true))

(fn UpdateSwimCameraState
  (params (Dive :type Boolean) (FastSwim :type Boolean) (Swom2Dive :type Boolean) (Dive2Swim :type Boolean) (Interact :type Boolean))
  (Variables|States|SetDive Dive)
  (Variables|States|SetFast FastSwim)
  (Variables|States|SetSwim%202Dive Swom2Dive)
  (Variables|States|SetDive%202Swim Dive2Swim)
  (Variables|States|SetInteract Interact)
  (return true))