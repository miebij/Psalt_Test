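; Anim notify for the swimming system that plays hand and foot water sounds from swimming, climb-out and shallow-water animations.
; Per-notify flags (hand, shallow, climbing, move, underwater, fast) select the sound spawned attached to a bone, while a state name overrides them for dive, drowning and jump splash.
; Shallow footsteps pass a vertical line-trace hit as their location.
; GetNotifyName builds the notify's label from the same settings.
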(fn ReceivedNotify
  (params (MeshComp :type Skeletal%20Mesh%20Component%20Object%20Reference) (Animation :type Anim%20Sequence%20Base%20Object%20Reference) (EventReference :type Anim%20Notify%20Event%20Reference%20Structure%20%28by%20ref%29))
  (LocalVariables|SetSoundLocation (|GetSoundLocation MeshComp))
  (Utilities|FlowControl|Sequence
    (:then_0
      (if (Utilities|Name|Equal(Name) (Variables|Default|GetUndefinedStateName) "None")
        (if (Variables|Default|GetHand)
          (if (not (Variables|Default|GetShallow))
            (if (Variables|Default|GetClimbing)
              ;[0.3333 0.2106 0.08914] Climb Out
              (Audio|SpawnSoundAttached (Variables|ClimbOut|GetClimbOutHandSound) MeshComp (Variables|Default|GetBoneName) "0, 0, 0" "0, 0, 0" "KeepRelativeOffset" true (Math|Float|MakeLiteralFloat 2.0) (Math|Float|MakeLiteralFloat 1.0) 0.0 0 0)
              (elif (Variables|Default|GetMove)
                (if (Variables|Default|GetUnderwater)
                  ;[0 0.1058 0.5729] Swim Underwater
                  (if (Variables|Default|GetFast)
                    (Audio|SpawnSoundAttached (Variables|Underwater|GetUW_SwimPushFastSound) MeshComp (Variables|Default|GetBoneName) "0, 0, 0" "0, 0, 0" "KeepRelativeOffset" true (Math|Float|MakeLiteralFloat 5.0) (Math|Float|MakeLiteralFloat 1.0) 0.0 0 0)
                    (else
                      (Audio|SpawnSoundAttached (Variables|Underwater|GetUW_SwimPushSound) MeshComp (Variables|Default|GetBoneName) "0, 0, 0" "0, 0, 0" "KeepRelativeOffset" true (Math|Float|MakeLiteralFloat 3.0) (Math|Float|MakeLiteralFloat 1.0) 0.0 0 0)))
                  (else
                    ;[0 0.4355 0.5729] Swim Surface
                    (if (Variables|Default|GetFast)
                      (Audio|SpawnSoundAttached (Variables|Surface|GetSF_SwimPushFastSound) MeshComp (Variables|Default|GetBoneName) "0, 0, 0" "0, 0, 0" "KeepRelativeOffset" true (Math|Float|MakeLiteralFloat 2.0) (Math|Float|MakeLiteralFloat 1.0) 0.0 0 0)
                      (else
                        (Audio|SpawnSoundAttached (Variables|Surface|GetSF_SwimPushSound) MeshComp (Variables|Default|GetBoneName) "0, 0, 0" "0, 0, 0" "KeepRelativeOffset" true (Math|Float|MakeLiteralFloat 2.0) (Math|Float|MakeLiteralFloat 1.0) 0.0 0 0)))))
                (else
                  ;[0 0.5729 0.4229] Swim Idle
                  (if (Variables|Default|GetUnderwater)
                    (Audio|SpawnSoundAttached (Variables|Underwater|GetUW_IdlePushSound) MeshComp (Variables|Default|GetBoneName) "0, 0, 0" "0, 0, 0" "KeepRelativeOffset" true (Math|Float|MakeLiteralFloat 4.0) (Math|Float|MakeLiteralFloat 1.0) 0.0 0 0)
                    (else
                      (Audio|SpawnSoundAttached (Variables|Surface|GetSF_IdlePushSound) MeshComp (Variables|Default|GetBoneName) "0, 0, 0" "0, 0, 0" "KeepRelativeOffset" true (Math|Float|MakeLiteralFloat 2.0) (Math|Float|MakeLiteralFloat 1.0) 0.0 0 0)))))))
          (elif (Variables|Default|GetShallow)
            ;[0.07859 0.3333 0.06469] Shallow Water
            (bind _impactpoint (CallFunction|FootTrace MeshComp))
            (Audio|SpawnSoundAttached (Variables|Misc|GetShallowWaterFootSound) MeshComp (Variables|Default|GetBoneName) _impactpoint "0, 0, 0" "KeepWorldPosition" true (Math|Float|MakeLiteralFloat 2.5) (Math|Float|MakeLiteralFloat 1.0) 0.0 0 0)
            (elif (Variables|Default|GetClimbing)
              ;[0.3333 0.2106 0.08914] Climb Out
              (Audio|SpawnSoundAttached (Variables|ClimbOut|GetClimbOutFootSound) MeshComp (Variables|Default|GetBoneName) "0, 0, 0" "0, 0, 0" "KeepRelativeOffset" true (Math|Float|MakeLiteralFloat 5.0) (Math|Float|MakeLiteralFloat 1.0) 0.0 0 0)
              (elif (Variables|Default|GetMove)
                (if (Variables|Default|GetUnderwater)
                  ;[0 0.1058 0.5729] Swim Underwater
                  (if (Variables|Default|GetFast)
                    (Audio|SpawnSoundAttached (Variables|Underwater|GetUW_SwimFastFootSound) MeshComp (Variables|Default|GetBoneName) "0, 0, 0" "0, 0, 0" "KeepRelativeOffset" true (Math|Float|MakeLiteralFloat 5.0) (Math|Float|MakeLiteralFloat 1.0) 0.0 0 0)
                    (else
                      (Audio|SpawnSoundAttached (Variables|Underwater|GetUW_SwimFootSound) MeshComp (Variables|Default|GetBoneName) "0, 0, 0" "0, 0, 0" "KeepRelativeOffset" true (Math|Float|MakeLiteralFloat 3.0) (Math|Float|MakeLiteralFloat 1.0) 0.0 0 0)))
                  (else
                    ;[0 0.4355 0.5729] Swim Surface
                    (if (Variables|Default|GetFast)
                      (Audio|SpawnSoundAttached (Variables|Surface|GetSF_SwimFastFootSound) MeshComp (Variables|Default|GetBoneName) "0, 0, 0" "0, 0, 0" "KeepRelativeOffset" true (Math|Float|MakeLiteralFloat 7.0) (Math|Float|MakeLiteralFloat 1.0) 0.0 0 0))))
                (else
                  ;[0 0.5729 0.4229] Swim Idle
                  (if (Variables|Default|GetUnderwater)
                    _))))))
        (elif (Utilities|Name|Equal(Name) (Variables|Default|GetUndefinedStateName) "DiveUnderwater")
          (Audio|SpawnSoundAttached (Variables|Misc|GetDiveUnderwaterSound) MeshComp (Variables|Default|GetBoneName) "0, 0, 0" "0, 0, 0" "KeepRelativeOffset" true (Math|Float|MakeLiteralFloat 3.0) (Math|Float|MakeLiteralFloat 1.0) 0.0 0 0)
          (elif (Utilities|Name|Equal(Name) (Variables|Default|GetUndefinedStateName) "Drowning")
            (Audio|SpawnSoundAttached (Variables|Misc|GetDrowningSound) MeshComp (Variables|Default|GetBoneName) "0, 0, 0" "0, 0, 0" "KeepRelativeOffset" true (Math|Float|MakeLiteralFloat 3.0) (Math|Float|MakeLiteralFloat 1.0) 0.0 0 0)
            (elif (Utilities|Name|Equal(Name) (Variables|Default|GetUndefinedStateName) "Jump")
              (Audio|SpawnSoundAttached (Variables|ClimbOut|GetClimbOutSplashSound) MeshComp (Variables|Default|GetBoneName) "0, 0, 0" "0, 0, 0" "KeepRelativeOffset" true (Math|Float|MakeLiteralFloat 5.0) (Math|Float|MakeLiteralFloat 1.0) 0.0 0 0))))))
    (:then_1
      (return false))))

(fn GetNotifyName
  (if (Utilities|Name|Equal(Name) (Variables|Default|GetUndefinedStateName) "None")
    (if (not (Variables|Default|GetShallow))
      (if (not (Variables|Default|GetClimbing))
        (return (Utilities|String|Append (Utilities|String|SelectString "UW" "SF" (Variables|Default|GetUnderwater)) (Utilities|String|SelectString "_Hand" "_Foot" (Variables|Default|GetHand)) (Utilities|String|SelectString "" "_Idle" (Variables|Default|GetMove)) (Utilities|String|SelectString "_Push" "" (Variables|Default|GetHand)) (Utilities|String|SelectString "_Fast" "" (Variables|Default|GetFast))))
        (else
          (return (Utilities|String|Append "Climb" (Utilities|String|SelectString "_Hand" "_Foot" (Variables|Default|GetHand))))))
      (else
        (return (Utilities|String|Append "Shallow" (Utilities|String|SelectString "_Hand" "_Foot" (Variables|Default|GetHand))))))
    (else
      (return (Utilities|String|ToString(Name) (Variables|Default|GetUndefinedStateName))))))

(fn FootTrace
  (params (Target :type Scene%20Component%20Object%20Reference))
  (bind _bonename (Variables|Default|GetBoneName))
  (bind _returnvalue (Transformation|GetSocketLocation Target _bonename))
  (bind (_outhit _returnvalue_2) (Collision|LineTraceByChannel (+ _returnvalue "0, 0,60.000000") (- _returnvalue "0, 0,60.000000") "TraceTypeQuery1" false 0 "None"))
  (if _returnvalue_2
    (return (.ImpactPoint (Collision|BreakHitResult _outhit)))
    (else
      (return (Transformation|GetSocketLocation Target (Variables|Default|GetBoneName))))))