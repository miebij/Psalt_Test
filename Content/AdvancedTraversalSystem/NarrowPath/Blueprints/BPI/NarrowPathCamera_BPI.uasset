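; Blueprint Interface for the narrow path camera in the Advanced Traversal System, defining the messages used to drive that camera.
; It declares functions to pass a character reference and to update blend alpha, target rotation, offset, FOV and camera state.
; It holds only signatures, so the camera behavior lives in whichever Blueprints implement it.
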(fn SetNarrowCameraCharRef
  (params (Character :type Actor%20Object%20Reference))
  (return false))

(fn UpdateAlpha
  (params (Alpha :type Float%20%28double-precision%29))
  (return false))

(fn UpdateNarrowCameraRotation
  (params (TargetRotation :type Rotator))
  (return false))

(fn UpdateNarrowCameraOffset
  (params (Offset :type Vector))
  (return false))

(fn UpdateNarrowCameraFOV
  (params (FOV :type Float%20%28double-precision%29))
  (return false))

(fn UpdateNarrowCameraState
  (params (State :type Integer))
  (return false))