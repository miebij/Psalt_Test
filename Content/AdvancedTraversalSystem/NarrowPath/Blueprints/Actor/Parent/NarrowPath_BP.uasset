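; Narrow path trigger actor for a traversal system, exposing camera, capsule, movement and animation settings through GetDatas.
; MainBox overlaps send enter messages to the overlapping actor's NarrowPathComponent, and an icon billboard can show at the nearest end.
; Exit messages fire from the inset BoxExit at unconnected ends or MainBox at connected ones, using StartConnect/EndConnect flags.
; Construction sizes BoxExit, removes it for OneShot paths, and draws optional debug lines.
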(event OnComponentBeginOverlap(MainBox)
  (params (OverlappedComponent :type Primitive%20Component%20Object%20Reference) (OtherActor :type Actor%20Object%20Reference) (OtherComp :type Primitive%20Component%20Object%20Reference) (OtherBodyIndex :type Integer) (bFromSweep :type Boolean) (SweepResult :type Hit%20Result%20Structure%20%28by%20ref%29))
  (bind _narrowpathcomponent (Variables|Default|GetNarrowPathComponent))
  (bind _returnvalue (Actor|GetComponentbyClass OtherActor _narrowpathcomponent))
  ;[0.1594 0.4792 0.1817] Enter
  (Variables|Default|SetbIn true)
  (Utilities|IsValid _returnvalue
    (:Is%20Valid
      (Class|NarrowPathBoxBPI|NarrowEnter(Message) _returnvalue self))))

(event OnComponentBeginOverlap(BoxExit)
  (params (OverlappedComponent :type Primitive%20Component%20Object%20Reference) (OtherActor :type Actor%20Object%20Reference) (OtherComp :type Primitive%20Component%20Object%20Reference) (OtherBodyIndex :type Integer) (bFromSweep :type Boolean) (SweepResult :type Hit%20Result%20Structure%20%28by%20ref%29))
  ;[0.1594 0.4792 0.1817] Enter
  (Variables|Default|SetbInnerBox true))

(event OnComponentEndOverlap(BoxExit)
  (params (OverlappedComponent :type Primitive%20Component%20Object%20Reference) (OtherActor :type Actor%20Object%20Reference) (OtherComp :type Primitive%20Component%20Object%20Reference) (OtherBodyIndex :type Integer))
  (bind _narrowpathcomponent (Variables|Default|GetNarrowPathComponent))
  (bind _returnvalue (Actor|GetComponentbyClass OtherActor _narrowpathcomponent))
  ;[0.4792 0.1848 0.1417] Exit
  (|It'sNotConnected OtherActor
    (:It's%20not%20connected
      (Variables|Default|SetbIn false)
      (Variables|Default|SetbInnerBox false)
      (Rendering|SetVisibility (Variables|Default|GetBillboardClose) false false)
      (Utilities|IsValid _returnvalue
        (:Is%20Valid
          (Class|NarrowPathBoxBPI|NarrowExit(Message) _returnvalue self))))))

(event OnComponentEndOverlap(MainBox)
  (params (OverlappedComponent :type Primitive%20Component%20Object%20Reference) (OtherActor :type Actor%20Object%20Reference) (OtherComp :type Primitive%20Component%20Object%20Reference) (OtherBodyIndex :type Integer))
  (bind _narrowpathcomponent (Variables|Default|GetNarrowPathComponent))
  (bind _returnvalue (Actor|GetComponentbyClass OtherActor _narrowpathcomponent))
  ;[0.4792 0.1848 0.1417] Exit
  (Class|NarrowPathBoxBPI|NarrowInteractionIcon(Message) self false OtherActor)
  (if (Variables|Default|GetbIn)
    (Variables|Default|SetbIn false)
    (|ItWasConnected OtherActor
      (:Exit%20was%20connected
        (Rendering|SetVisibility (Variables|Default|GetBillboardClose) false false)
        (Utilities|IsValid _returnvalue
          (:Is%20Valid
            (Class|NarrowPathBoxBPI|NarrowExit(Message) _returnvalue self)))))))

(event EventBeginPlay)

(event Collision|EventActorBeginOverlap
  (params (OtherActor :type Actor%20Object%20Reference)))

(event EventTick
  (params (DeltaSeconds :type Float%20%28single-precision%29)))

(event EventNarrowInteractionIcon
  (params (Show :type Boolean) (Actor :type Actor%20Object%20Reference))
  ;[0.0766 0.363 0.4792] Interaction Icon
  (if Show
    (Variables|Default|SetbIn true)
    (bind _enterpoint (CallFunction|GetPoints Actor))
    (Transformation|SetWorldLocation (Variables|Default|GetBillboardClose) (|InteractionIconLocation _enterpoint) false false)
    (Rendering|SetVisibility (Variables|Default|GetBillboardClose) true false)
    (else
      (Rendering|SetVisibility (Variables|Default|GetBillboardClose) false false))))

(fn ConstructionScript
  (bind _returnvalue (Transformation|GetActorScale3D))
  (bind (_x _y _z) (Math|Vector|BreakVector _returnvalue))
  (Rendering|Components|Sprite|SetSprite (Variables|Default|GetBillboardClose) (Variables|Default|GetIconSprite))
  (if (Variables|Default|GetbOneShot)
    (Components|DestroyComponent (Variables|Default|GetBoxExit)))
  (bind (_end _start) (CallFunction|GetBoxStartEndPoints))
  (|DebugConnects _end _start)
  (|DebugStartOffsets _end _start)
  (Transformation|SetWorldScale3D (Variables|Default|GetBoxExit) (Math|Vector|MakeVector (/ (- (/ (Math|Vector|VectorLength (- _end _start)) 2.0) (Variables|Default|GetExitOffsetY)) 32.0) _y _z))
  (Transformation|SetWorldScale3D (Variables|Default|GetArrow) (/ (Transformation|GetWorldScale (Variables|Default|GetArrow)) (Transformation|GetActorScale3D))))

(fn GetPoints
  (params (Target :type Actor%20Object%20Reference))
  (bind _returnvalue (Transformation|GetActorLocation Target))
  (bind (_end _start) (CallFunction|GetBoxStartEndPoints))
  (if (<= (Math|Vector|VectorLength (- _end _returnvalue)) (Math|Vector|VectorLength (- _start _returnvalue)))
    (LocalVariables|SetEnterPoint-Local _end)
    (LocalVariables|SetExitPoint-Local _start)
    (else
      (LocalVariables|SetEnterPoint-Local _start)
      (LocalVariables|SetExitPoint-Local _end)))
  (return (LocalVariables|GetExitPoint-Local) (LocalVariables|GetEnterPoint-Local)))

(fn GetBoxStartEndPoints
  (bind _returnvalue (Transformation|GetActorForwardVector))
  (bind _mainbox (Variables|Default|GetMainBox))
  (bind _mainbox_2 (Variables|Default|GetMainBox))
  (bind _returnvalue_2 (Transformation|GetWorldScale _mainbox))
  (bind _returnvalue_3 (Transformation|GetWorldLocation _mainbox_2))
  (bind _x (Math|Vector|BreakVector _returnvalue_2))
  (bind _returnvalue_4 (* _x 32.0))
  (return (+ _returnvalue_3 (* _returnvalue _returnvalue_4)) (+ _returnvalue_3 (* _returnvalue (* _returnvalue_4 -1.0)))))

(fn GetDatas
  (return (Variables|Default|GetbOneShot) (Variables|Default|GetbUseEnterMontage) (Variables|Default|GetbUseExitMontage) (Variables|Default|GetbUseInpuKey) (Variables|Default|GetbRightSide) (Variables|Default|GetbMirrorSide) (Variables|Default|GetFixCamera) (Variables|Default|GetChangeCapsuleRadius) (Variables|Default|GetCapsuleRadius) (Variables|Default|GetCameraOffset) (Variables|Default|GetFOV) (Variables|Default|GetCharacterOffsetX) (Variables|Default|GetEnterOffsetY) (Variables|Default|GetWalkSpeed) (Variables|Default|GetAnimType)))