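; Blueprint Interface for the zipline climbing camera in the Advanced Traversal System.
; It declares calls to bind the character, player camera and controller, then update climb state (move-to, aiming), camera data, alpha, rotation, offset and FOV.
; Further calls add or remove the climbing camera with blend times, or reset it.
; It holds only function signatures, so implementers supply the camera behavior.
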(fn SetZiplineCameraCharRef
  (params (Character :type Actor%20Object%20Reference) (PlayerCamera :type Player%20Camera%20Manager%20Object%20Reference) (PlayerController :type Player%20Controller%20Object%20Reference))
  (return false))

(fn UpdateZiplineClimbCameraState
  (params (MoveTo :type Boolean) (Aiming :type Boolean))
  (return false))

(fn UpdateZiplineClimbCameraDatas
  (return false))

(fn UpdateZiplineClimbAlpha
  (params (Alpha :type Float%20%28double-precision%29))
  (return false))

(fn UpdateZiplineClimbCameraRotation
  (params (TargetRotation :type Rotator))
  (return false))

(fn UpdateZiplineClimbCameraOffset
  (params (Offset :type Vector))
  (return false))

(fn UpdateZiplineClimbCameraFOV
  (params (FOV :type Float%20%28double-precision%29))
  (return false))

(fn AddZiplineClimbingCamera
  (params (BlendInTime :type Float%20%28double-precision%29))
  (return false))

(fn RemoveZiplineClimbingCamera
  (params (BlendOutTime :type Float%20%28double-precision%29))
  (return false))

(fn ResetZiplineClimbingCamera
  (return false))