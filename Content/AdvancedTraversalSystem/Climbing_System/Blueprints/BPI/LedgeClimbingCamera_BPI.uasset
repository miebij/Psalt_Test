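; Blueprint interface for the ledge climbing camera in the Advanced Traversal System, declaring the calls that drive it during climbing.
; It takes character, camera and controller references, then receives climb state flags such as move-to, freehang, corner, turn back, aiming and side switch.
; Further calls update camera data, alpha, rotation, offset and FOV, and add, remove or reset the camera, with timed blend in and out.
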(fn SetLedgeClimbCameraCharRef
  (params (Character :type Actor%20Object%20Reference) (PlayerCamera :type Player%20Camera%20Manager%20Object%20Reference) (PlayerController :type Player%20Controller%20Object%20Reference))
  (return false))

(fn UpdateLedgeClimbCameraState
  (params (MoveTo :type Boolean) (Freehang :type Boolean) (Corner :type Boolean) (TurnBack :type Boolean) (Aiming :type Boolean) (SwitchSide :type Boolean))
  (return false))

(fn UpdateLedgeClimbCameraDatas
  (return false))

(fn UpdateLedgeClimbAlpha
  (params (Alpha :type Float%20%28double-precision%29))
  (return false))

(fn UpdateLedgeClimbCameraRotation
  (params (TargetRotation :type Rotator))
  (return false))

(fn UpdateLedgeClimbCameraOffset
  (params (Offset :type Vector))
  (return false))

(fn UpdateLedgeClimbCameraFOV
  (params (FOV :type Float%20%28double-precision%29))
  (return false))

(fn AddLedgeClimbingCamera
  (params (BlendInTime :type Float%20%28double-precision%29))
  (return false))

(fn RemoveLedgeClimbingCamera
  (params (BlendOutTime :type Float%20%28double-precision%29))
  (return false))

(fn ResetLedgeClimbingCamera
  (return false))