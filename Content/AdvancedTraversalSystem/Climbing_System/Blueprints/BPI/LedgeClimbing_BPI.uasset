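; Blueprint interface for the ledge climbing system, declaring the messages that pass climbing state between implementers.
; Most functions push states such as hanging, shimmy, reach, corners, ledge jumps and aiming, plus speed multipliers and hand, foot and pelvis IK data.
; Others relay hand notifies, activation, physics, overlay and camera changes.
; A few return values for input, overlay, grab disabling, external start/finish and ledge collection.
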(fn EnableClimbingSystem
  (params (Enable_Climbing :type Boolean) (BlendIn :type Float%20%28double-precision%29) (BlendOut :type Float%20%28double-precision%29)))

(fn EnableFreehang
  (params (FreeHanging :type Boolean) (bIsBlocked :type Boolean)))

(fn States
  (params (GrabLedge :type Boolean) (GrabAngle :type Float%20%28double-precision%29) (Hanging :type Boolean)))

(fn Shimmy
  (params (MovingRight :type Boolean) (MovingLeft :type Boolean)))

(fn Reach
  (params (can_Reach :type Boolean) (ReachAngle :type Float%20%28double-precision%29) (ReachSide :type Float%20%28double-precision%29)))

(fn TurnCorner
  (params (TurnRight :type Boolean) (TurnLeft :type Boolean) (OuterCorner :type Boolean) (InnerCorner :type Boolean)))

(fn TurnBack
  (params (TurnBack :type Boolean)))

(fn SwitchLedgeSide
  (params (SwitchSide :type Boolean)))

(fn Climb/JumptoLedge
  (params (JumpToLedge :type Boolean) (ClimbToLedge :type Boolean) (Angle :type Float%20%28double-precision%29) (Distance :type Float%20%28double-precision%29) (Side :type Float%20%28double-precision%29)))

(fn ClimbDowntoLedge
  (params (Climb_Down_Ledge :type Boolean))
  (return))

(fn AutoMovement
  (params (bAutoMovement :type Boolean)))

(fn ReleaseLedge
  (params (ReleaseLedge :type Boolean)))

(fn LedgeFreeJump
  (params (bFreeJumping :type Boolean) (FreeJumpAngle :type Float%20%28double-precision%29) (FreeJumpSide :type Float%20%28double-precision%29) (FreeJumpVelocity :type Float%20%28double-precision%29) (Backward :type Boolean)))

(fn LedgeExternal
  (params (ClimbingExternalIn :type Boolean) (ClimbingExternalOut :type Boolean) (AngleExt :type Float%20%28double-precision%29) (SideExt :type Float%20%28double-precision%29) (DistanceExt :type Float%20%28double-precision%29)))

(fn LedgeClimbAimingStates
  (params (UseOverlay :type Boolean) (Aiming :type Boolean) (Ready :type Boolean) (Stand :type Boolean) (AimingingRotation :type Rotator)))

(fn LedgeClimbingInput
  (params (MoveRight :type Float%20%28double-precision%29) (MoveForward :type Float%20%28double-precision%29)))

(fn PelvisOffsetUpdate
  (params (PelvisOffset :type Vector)))

(fn SpeedMultiplier
  (params (GrabMultiplier :type Float%20%28double-precision%29) (ShimmyMultiplier :type Float%20%28double-precision%29) (ClimbMultiplier :type Float%20%28double-precision%29) (JumpMultiplier :type Float%20%28double-precision%29) (JumpBackwardMultiplier :type Float%20%28double-precision%29) (CornerMultiplier :type Float%20%28double-precision%29) (ClimbTimeRatio :type Float%20%28double-precision%29)))

(fn CurrentHandIK
  (params (Hand_R :type Vector) (Hand_L :type Vector) (Hand_R_Rot :type Rotator) (Hand_L_Rot :type Rotator)))

(fn NewHandIK
  (params (Hand_R :type Vector) (Hand_L :type Vector) (Hand_R_Rot :type Rotator) (Hand_L_Rot :type Rotator)))

(fn HandTracesMovement
  (params (ImpactPointRight :type Vector) (RightHandOffset :type Vector) (RightHandRotation :type Rotator) (ImpactPointLeft :type Vector) (LeftHandOffset :type Vector) (LeftHandRotation :type Rotator)))

(fn CurrentLegIK
  (params (Foot_R :type Vector) (Foot_L :type Vector) (Foot_r_Rot :type Rotator) (Foot_L_Rot :type Rotator)))

(fn AnimNotifyHandR)

(fn AnimNotifyHandL)

(fn LedgeClimbingActivated/Deactivated
  (params (Actived/Deactivated :type Boolean)))

(fn LedgeClimbingMovementState
  (params (State :type Byte)))

(fn LedgeClimbingPhysicsActivated/Deactivated
  (params (Activated/Deactivated :type Boolean)))

(fn LedgeClimbOverlayResponse
  (params (Disable :type Boolean)))

(fn LedgeSwitchCamera
  (params (Right :type Boolean)))

(fn DisableLedgeGrab
  (return false))

(fn LedgeClimbingInputs
  (return 0.0 0.0))

(fn LedgeClimbOverlay
  (return false 0 false))

(fn LedgeFinishExt
  (return false))

(fn LedgeStartExt
  (params (Index :type Integer) (HorizontalMovement :type Boolean) (PreDelay :type Float%20%28double-precision%29) (MovementTime :type Float%20%28double-precision%29))
  (return false))

(fn LedgeGobalCollect
  (params (SearchLocation :type Vector) (Radius :type Float%20%28double-precision%29))
  (return false))