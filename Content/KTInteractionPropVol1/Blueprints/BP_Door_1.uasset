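; BP_Door_1 is an interactable double door that player 0 toggles with E, with input enabled while something overlaps TriggerBoxR.
; The Open timeline plays or reverses with a sound at world origin, yawing DoorR and DoorL in opposite directions and rolling Lever.
; IaPull selects the OpenPull track instead of Open for the doors.
; Tick hides both UI components while the timeline plays.
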(event OnComponentBeginOverlap(TriggerBoxR)
  (params (OverlappedComponent :type Primitive%20Component%20Object%20Reference) (OtherActor :type Actor%20Object%20Reference) (OtherComp :type Primitive%20Component%20Object%20Reference) (OtherBodyIndex :type Integer) (bFromSweep :type Boolean) (SweepResult :type Hit%20Result%20Structure%20%28by%20ref%29))
  (Input|EnableInput (Game|GetPlayerController 0)))

(event OnComponentEndOverlap(TriggerBoxR)
  (params (OverlappedComponent :type Primitive%20Component%20Object%20Reference) (OtherActor :type Actor%20Object%20Reference) (OtherComp :type Primitive%20Component%20Object%20Reference) (OtherBodyIndex :type Integer))
  (Input|DisableInput (Game|GetPlayerController 0)))

(event EventBeginPlay)

(event Collision|EventActorBeginOverlap
  (params (OtherActor :type Actor%20Object%20Reference)))

(event EventTick
  (params (DeltaSeconds :type Float%20%28single-precision%29))
  (if (Audio|Components|Audio|IsPlaying (Variables|Default|GetOpen))
    (CallFunction|SetUI true)
    (else
      (CallFunction|SetUI false))))

(event Input|KeyboardEvents|E
  (params (Key :type Key%20Structure))
  (:Pressed
    (if (Variables|Default|GetIsOpen)
      (Variables|Default|SetIsOpen false)
      (Audio|PlaySoundatLocation (Variables|Default|GetCloseSound) "0, 0, 0" "0, 0, 0" 1.0 1.0 0.0 0 0 0 0)
      (bind (_direction _open _openpull) (Timeline|Open Reverse)
        (:Update
          (Transformation|SetActorRotation (Variables|Default|GetLever) (Math|Rotator|MakeRotator (* _open 0.5) 0.0 0.0))
          (if (Variables|Default|GetIaPull)
            (Transformation|SetRelativeRotation (Variables|Default|GetDoor_R) (Math|Rotator|MakeRotator 0.0 0.0 _openpull) false false)
            (Transformation|SetRelativeRotation (Variables|Default|GetDoor_L) (Math|Rotator|MakeRotator 0.0 0.0 (* _openpull -1.0)) false false)
            (else
              (Transformation|SetRelativeRotation (Variables|Default|GetDoor_R) (Math|Rotator|MakeRotator 0.0 0.0 _open) false false)
              (Transformation|SetRelativeRotation (Variables|Default|GetDoor_L) (Math|Rotator|MakeRotator 0.0 0.0 (* _open -1.0)) false false)))))
      (else
        (Variables|Default|SetIsOpen true)
        (Audio|PlaySoundatLocation (Variables|Default|GetOpenSound) "0, 0, 0" "0, 0, 0" 1.0 1.0 0.0 0 0 0 0)
        (Timeline|Open Play)))))

(fn ConstructionScript)

(fn SetUI
  (params (Hidden :type Boolean))
  (Development|SetHiddeninGame (Variables|Default|GetUI) Hidden false)
  (Development|SetHiddeninGame (Variables|Default|GetUI1) Hidden false))