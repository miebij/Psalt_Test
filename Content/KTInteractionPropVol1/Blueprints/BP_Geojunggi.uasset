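; Interactive Geojunggi lift prop that a player toggles between raised and lowered with the interact input or E key.
; Two trigger boxes enable and disable input for the overlapping ALS character's controller.
; Each toggle, blocked during animation, plays the skeletal animation and sound, calls LiftBP, and runs the Rope timeline forward or backward to scroll the rope material's OffsetV.
; Tick hides the UI components while the animation plays.
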(event OnComponentBeginOverlap(TriggerBoxR)
  (params (OverlappedComponent :type Primitive%20Component%20Object%20Reference) (OtherActor :type Actor%20Object%20Reference) (OtherComp :type Primitive%20Component%20Object%20Reference) (OtherBodyIndex :type Integer) (bFromSweep :type Boolean) (SweepResult :type Hit%20Result%20Structure%20%28by%20ref%29))
  (bind _asals_anim_man_character_bp (Utilities|Casting|CastToALS_AnimMan_CharacterBP OtherActor))
  (Input|EnableInput (Pawn|GetLocalViewingPlayerController _asals_anim_man_character_bp)))

(event OnComponentEndOverlap(TriggerBoxR)
  (params (OverlappedComponent :type Primitive%20Component%20Object%20Reference) (OtherActor :type Actor%20Object%20Reference) (OtherComp :type Primitive%20Component%20Object%20Reference) (OtherBodyIndex :type Integer))
  (bind _asals_anim_man_character_bp (Utilities|Casting|CastToALS_AnimMan_CharacterBP OtherActor))
  (Input|DisableInput (Pawn|GetLocalViewingPlayerController _asals_anim_man_character_bp)))

(event OnComponentBeginOverlap(TriggerBoxL)
  (params (OverlappedComponent :type Primitive%20Component%20Object%20Reference) (OtherActor :type Actor%20Object%20Reference) (OtherComp :type Primitive%20Component%20Object%20Reference) (OtherBodyIndex :type Integer) (bFromSweep :type Boolean) (SweepResult :type Hit%20Result%20Structure%20%28by%20ref%29))
  (bind _asals_anim_man_character_bp (Utilities|Casting|CastToALS_AnimMan_CharacterBP OtherActor))
  (Input|EnableInput (Pawn|GetLocalViewingPlayerController _asals_anim_man_character_bp)))

(event OnComponentEndOverlap(TriggerBoxL)
  (params (OverlappedComponent :type Primitive%20Component%20Object%20Reference) (OtherActor :type Actor%20Object%20Reference) (OtherComp :type Primitive%20Component%20Object%20Reference) (OtherBodyIndex :type Integer))
  (bind _asals_anim_man_character_bp (Utilities|Casting|CastToALS_AnimMan_CharacterBP OtherActor))
  (Input|DisableInput (Pawn|GetLocalViewingPlayerController _asals_anim_man_character_bp)))

(event Input|EnhancedActionEvents|EnhancedInputActionIA_ALS_Interact
  (params (ActionValue :type Boolean) (ElapsedSeconds :type Float%20%28double-precision%29) (TriggeredSeconds :type Float%20%28double-precision%29) (InputAction :type Input%20Action%20Object%20Reference :default "/Game/AdvancedLocomotionV4/Blueprints/CharacterLogic/Inputs/IA_ALS_Interact.IA_ALS_Interact"))
  (bind _skm_geojunggi (Variables|Default|GetSKM_Geojunggi))
  (bind _liftbp (Variables|Default|GetLiftBP))
  (:Triggered
    (if (not (Audio|Components|Audio|IsPlaying _skm_geojunggi)) :!label _label
      (if (Variables|Default|GetIsDown)
        (Components|Animation|PlayAnimation _skm_geojunggi "/Game/KTInteractionPropVol1/Animation/ANIM_Geojunggi_LiftUp.ANIM_Geojunggi_LiftUp" false)
        (Default|GoUP _liftbp)
        (Audio|PlaySoundatLocation "/Game/KTInteractionPropVol1/Sound/Sound_Geojunggi_LiftUp.Sound_Geojunggi_LiftUp" "0, 0, 0" "0, 0, 0" 1.0 1.0 0.0 0 0 0 0)
        (Variables|Default|SetIsDown false)
        (bind _liftup (Timeline|Rope Play)
          (:Update
            (Rendering|Material|SetScalarParameterValue (Variables|Default|GetMi_Rope) "OffsetV" _liftup :!class /Script/Engine.MaterialInstanceDynamic)))
        (else
          (Components|Animation|PlayAnimation _skm_geojunggi "/Game/KTInteractionPropVol1/Animation/ANIM_Geojunggi_LiftDown.ANIM_Geojunggi_LiftDown" false)
          (Default|GoDown _liftbp)
          (Audio|PlaySoundatLocation "/Game/KTInteractionPropVol1/Sound/Sound_Geojunggi_LiftDown.Sound_Geojunggi_LiftDown" "0, 0, 0" "0, 0, 0" 1.0 1.0 0.0 0 0 0 0)
          (Variables|Default|SetIsDown true)
          (Timeline|Rope Reverse)))))
  (:Started
    (goto _label)))

(event EventBeginPlay
  (bind _returnvalue (Rendering|Material|CreateDynamicMaterialInstance (Variables|Default|GetSKM_Geojunggi) 0 "/Game/KTInteractionPropVol1/Material/M_Rope.M_Rope" "OffsetV" :!class /Script/Engine.PrimitiveComponent))
  (Variables|Default|SetMi_Rope _returnvalue))

(event Collision|EventActorBeginOverlap
  (params (OtherActor :type Actor%20Object%20Reference)))

(event EventTick
  (params (DeltaSeconds :type Float%20%28single-precision%29))
  (if (Audio|Components|Audio|IsPlaying (Variables|Default|GetSKM_Geojunggi))
    (CallFunction|SetUI true)
    (else
      (CallFunction|SetUI false))))

(event Input|KeyboardEvents|E
  (params (Key :type Key%20Structure :default "None"))
  (bind _skm_geojunggi (Variables|Default|GetSKM_Geojunggi))
  (bind _liftbp (Variables|Default|GetLiftBP))
  (:Pressed
    (if (not (Audio|Components|Audio|IsPlaying _skm_geojunggi))
      (if (Variables|Default|GetIsDown)
        (Components|Animation|PlayAnimation _skm_geojunggi "/Game/KTInteractionPropVol1/Animation/ANIM_Geojunggi_LiftUp.ANIM_Geojunggi_LiftUp" false)
        (Default|GoUP _liftbp)
        (Audio|PlaySoundatLocation "/Game/KTInteractionPropVol1/Sound/Sound_Geojunggi_LiftUp.Sound_Geojunggi_LiftUp" "0, 0, 0" "0, 0, 0" 1.0 1.0 0.0 0 0 0 0)
        (Variables|Default|SetIsDown false)
        (bind _liftup (Timeline|Rope Play)
          (:Update
            (Rendering|Material|SetScalarParameterValue (Variables|Default|GetMi_Rope) "OffsetV" _liftup :!class /Script/Engine.MaterialInstanceDynamic)))
        (else
          (Components|Animation|PlayAnimation _skm_geojunggi "/Game/KTInteractionPropVol1/Animation/ANIM_Geojunggi_LiftDown.ANIM_Geojunggi_LiftDown" false)
          (Default|GoDown _liftbp)
          (Audio|PlaySoundatLocation "/Game/KTInteractionPropVol1/Sound/Sound_Geojunggi_LiftDown.Sound_Geojunggi_LiftDown" "0, 0, 0" "0, 0, 0" 1.0 1.0 0.0 0 0 0 0)
          (Variables|Default|SetIsDown true)
          (Timeline|Rope Reverse))))))

(fn ConstructionScript)

(fn SetUI
  (params (Hidden :type Boolean))
  (Development|SetHiddeninGame (Variables|Default|GetUI) Hidden false)
  (Development|SetHiddeninGame (Variables|Default|GetUI1) Hidden false)
  (Development|SetHiddeninGame (Variables|Default|GetUI2) Hidden false)
  (Development|SetHiddeninGame (Variables|Default|GetUI3) Hidden false))