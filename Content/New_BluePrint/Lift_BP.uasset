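; Lift Blueprint that raises and lowers a Lift actor and scales its Ropes to follow the movement.
; GoUP and GoDown set the Movingup flag, which Tick reads every frame to play or reverse a Timeline.
; The Timeline interpolates the lift's Z between AT and BT, keeping X and Y, while a separate track drives the ropes' relative Z scale.
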(event Custom|GoUP
  (Variables|Default|Setmovingup true))

(event Custom|GoDown
  (Variables|Default|Setmovingup false))

(event EventBeginPlay)

(event Collision|EventActorBeginOverlap
  (params (OtherActor :type Actor%20Object%20Reference)))

(event EventTick
  (params (DeltaSeconds :type Float%20%28single-precision%29))
  (bind _lift (Variables|Default|Getlift))
  (bind _returnvalue (Transformation|GetActorLocation _lift))
  (if (Variables|Default|Getmovingup)
    (bind (_direction _newtrack_3 _newtrack_0) (Timeline|Timeline Play)
      (:Update
        (Transformation|SetActorLocation _lift (Math|Vector|MakeVector (.x _returnvalue) (.y _returnvalue) (+ (- (Variables|Default|GetAT) (* (Variables|Default|GetAT) _newtrack_3)) (* (Variables|Default|GetBT) _newtrack_3))) false false)
        (Transformation|SetActorRelativeScale3D (Variables|Default|GetRopes) (Math|Vector|MakeVector 1.0 1.0 _newtrack_0))))
    (else
      (Timeline|Timeline Reverse))))

(fn ConstructionScript)